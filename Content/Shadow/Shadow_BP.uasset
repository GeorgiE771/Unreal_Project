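; Shadow puzzle actor that the player rotates into a target orientation to earn the third key.
; Pressing E inside its box blends the view to the actor and redirects look input to pitch and roll the static mesh; pressing E again exits.
; Tick checks the mesh's world rotation against tolerance ranges.
; On a match it restores player control, disables the box, sets ThirdKey and marks itself complete.
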(event `self.ReceiveTick`
  (params (DeltaSeconds :type "Float (single-precision)"))
  (bind _returnvalue (`GameplayStatics.GetPlayerController` 0))
  (bind _returnvalue_2 (`GameplayStatics.GetPlayerController` 0))
  (if (not (`self.Is_complete`))
    (`|ExecutionSequence`
      (:`then_0`
        (if (`self.is_in`)
          (bind _asfirst_person_character (cast `/Game/FirstPersonBP/Blueprints/FirstPersonCharacter` (`GameplayStatics.GetPlayerCharacter` 0)))
          (if (`/Game/FirstPersonBP/Blueprints/FirstPersonCharacter.Is_pressed_E` _asfirst_person_character)
            (`self.EnableInput` _returnvalue_2)
            (`PlayerController.SetViewTargetWithBlend` _returnvalue_2 self 1.0 "VTBlend_Linear" 0.0 false)
            (`Controller.SetIgnoreMoveInput` _returnvalue_2 true)
            (`Controller.SetIgnoreLookInput` _returnvalue_2 true)
            (`KismetSystemLibrary.Delay` 1.0)
            (set `self.is_in` false))))
      (:`then_1`
        (bind _is_right (`self.Check`))
        (if _is_right
          (`self.DisableInput` _returnvalue_2)
          (`PrimitiveComponent.SetCollisionEnabled` (`self.Box  `) "NoCollision")
          (bind _asfirst_person_character_2 (cast `/Game/FirstPersonBP/Blueprints/FirstPersonCharacter` (`GameplayStatics.GetPlayerCharacter` 0)))
          (`PlayerController.SetViewTargetWithBlend` _returnvalue _asfirst_person_character_2 1.0 "VTBlend_Linear" 0.0 false)
          (`Controller.ResetIgnoreMoveInput` _returnvalue)
          (`Controller.ResetIgnoreLookInput` _returnvalue)
          (bind _asfirst_person_character_3 (cast `/Game/FirstPersonBP/Blueprints/FirstPersonCharacter` (`GameplayStatics.GetPlayerCharacter` 0)))
          (set `/Game/FirstPersonBP/Blueprints/FirstPersonCharacter.Third_Key` true _asfirst_person_character_3)
          (`KismetSystemLibrary.PrintString` "Key 3")
          (set `self.Is_complete` true)
          (`KismetSystemLibrary.Delay` 1.0)
          (set `self.is_in` false))))))

(event `self.Box  .OnComponentBeginOverlap`
  (params (OverlappedComponent :type "PrimitiveComponent Object Reference") (OtherActor :type "Actor Object Reference") (OtherComp :type "PrimitiveComponent Object Reference") (OtherBodyIndex :type Integer) (bFromSweep :type Boolean) (SweepResult :type "HitResult Structure (by ref)"))
  (set `self.is_in` true))

(event `self.Box  .OnComponentEndOverlap`
  (params (OverlappedComponent :type "PrimitiveComponent Object Reference") (OtherActor :type "Actor Object Reference") (OtherComp :type "PrimitiveComponent Object Reference") (OtherBodyIndex :type Integer))
  (set `self.is_in` false))

(event `Key|E`
  (params (Key :type "Key Structure"))
  (bind _returnvalue (`GameplayStatics.GetPlayerController` 0))
  (:`Pressed`
    (bind _asfirst_person_character (cast `/Game/FirstPersonBP/Blueprints/FirstPersonCharacter` (`GameplayStatics.GetPlayerCharacter` 0)))
    (`self.DisableInput` _returnvalue)
    (`PlayerController.SetViewTargetWithBlend` _returnvalue _asfirst_person_character 1.0 "VTBlend_Linear" 0.0 false)
    (`Controller.ResetIgnoreMoveInput` _returnvalue)
    (`Controller.ResetIgnoreLookInput` _returnvalue)
    (`KismetSystemLibrary.Delay` 1.0)
    (set `self.is_in` true)))

(event `InputAxis|Turn` :overrideparent false
  (params (AxisValue :type "Float (single-precision)"))
  (`self.Rotate Pitch` AxisValue))

(event `InputAxis|LookUp`
  (params (AxisValue :type "Float (single-precision)"))
  (`self.Rotate Roll` AxisValue))

(fn `Check`
  (returns (is_right :type Boolean))
  (bind (_returnvalue_roll _returnvalue_pitch _returnvalue_yaw) (`KismetMathLibrary.BreakRotator` (`SceneComponent.K2_GetComponentRotation` (`self.StaticMesh`))))
  (return (and (`KismetMathLibrary.InRange_FloatFloat` _returnvalue_yaw -95.0 -75.0) (`KismetMathLibrary.InRange_FloatFloat` _returnvalue_pitch -4.0 16.0) (`KismetMathLibrary.InRange_FloatFloat` _returnvalue_roll 70.0 90.0))))

(fn `Rotate Pitch`
  (params (rotate_pitch :type "Float (double-precision)"))
  (bind _staticmesh (`self.StaticMesh`))
  (`SceneComponent.K2_SetWorldRotation` _staticmesh (`KismetMathLibrary.ComposeRotators` (`KismetMathLibrary.MakeRotator` 0.0 rotate_pitch) (`SceneComponent.K2_GetComponentRotation` _staticmesh)) false false))

(fn `Rotate Roll`
  (params (rotate_roll :type "Float (double-precision)"))
  (bind _staticmesh (`self.StaticMesh`))
  (`SceneComponent.K2_SetWorldRotation` _staticmesh (`KismetMathLibrary.ComposeRotators` (`KismetMathLibrary.MakeRotator` rotate_roll) (`SceneComponent.K2_GetComponentRotation` _staticmesh)) false false))

(fn `UserConstructionScript`)