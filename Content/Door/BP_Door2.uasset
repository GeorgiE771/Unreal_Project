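; BP_Door2 is a key-locked swinging door that opens for a FirstPersonCharacter holding the FirstKey flag.
; Entering the Box trigger plays DoorTimeline, whose track drives the Door's relative yaw each update.
; Leaving the trigger with the key reverses the timeline to swing the door shut.
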(event `self.Box.OnComponentBeginOverlap`
  (params (OverlappedComponent :type "PrimitiveComponent Object Reference") (OtherActor :type "Actor Object Reference") (OtherComp :type "PrimitiveComponent Object Reference") (OtherBodyIndex :type Integer) (bFromSweep :type Boolean) (SweepResult :type "HitResult Structure (by ref)"))
  (bind _asfirst_person_character (cast `/Game/FirstPersonBP/Blueprints/FirstPersonCharacter` OtherActor))
  (if (`/Game/FirstPersonBP/Blueprints/FirstPersonCharacter.First_key` _asfirst_person_character)
    (bind (_direction _newtrack_0) (`Timeline|DoorTimeline` :!label _label)
      (:`Update`
        (`SceneComponent.K2_SetRelativeRotation` (`self.Door`) (`KismetMathLibrary.MakeRotator` 0.0 0.0 _newtrack_0) false false)))))

(event `self.Box.OnComponentEndOverlap`
  (params (OverlappedComponent :type "PrimitiveComponent Object Reference") (OtherActor :type "Actor Object Reference") (OtherComp :type "PrimitiveComponent Object Reference") (OtherBodyIndex :type Integer))
  (bind _asfirst_person_character (cast `/Game/FirstPersonBP/Blueprints/FirstPersonCharacter` OtherActor))
  (if (`/Game/FirstPersonBP/Blueprints/FirstPersonCharacter.First_key` _asfirst_person_character)
    (goto _label :!via `Reverse`)))

(fn `UserConstructionScript`)